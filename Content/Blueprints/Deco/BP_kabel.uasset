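; Decorative cable actor built along an editable spline in the construction script, with no active runtime logic.
; It adds a connector static mesh at the spline points, aligned to each point's rotation.
; A spline mesh component bends the main mesh between each pair of neighbouring points, using their tangents and the start point's up vector.
; Connector and cable meshes and their materials come from variables.
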(fn `UserConstructionScript`
  (bind _spline (`self.Spline`))
  (bind _spline_2 (`self.Spline`))
  (bind _spline_3 (`self.Spline`))
  (`|ExecutionSequence`
    (:`then_0`
      (for _index (range (+ (`SplineComponent.GetNumberOfSplinePoints` (`self.Spline`)) 1))
        (bind _returnvalue (`AddComponent|NODE_AddStaticMeshComponent-0` :`RelativeTransform` (`KismetMathLibrary.MakeTransform` (`SplineComponent.GetLocationAtSplinePoint` _spline _index "Local") (`SplineComponent.GetRotationAtSplinePoint` _spline _index "Local"))))
        (`StaticMeshComponent.SetStaticMesh` _returnvalue (`self.Connector Mesh`))
        (`PrimitiveComponent.SetMaterial` _returnvalue 0 (`self.ConnectorMeshMat`))))
    (:`then_1`
      (for _index_2 (range (+ (- (`SplineComponent.GetNumberOfSplinePoints` (`self.Spline`)) 2) 1))
        (bind _returnvalue_2 (`AddComponent|NODE_AddSplineMeshComponent-2`))
        (`StaticMeshComponent.SetStaticMesh` _returnvalue_2 (`self.MainMesh`))
        (`SplineMeshComponent.SetSplineUpDir` _returnvalue_2 (`KismetMathLibrary.GetUpVector` (`SplineComponent.GetRotationAtSplinePoint` (`self.Spline`) _index_2 "Local")) true)
        (`PrimitiveComponent.SetMaterial` _returnvalue_2 0 (`self.MainMeshMat`))
        (bind _returnvalue_3 (+ _index_2 1))
        (`SplineMeshComponent.SetStartAndEnd` _returnvalue_2 (`SplineComponent.GetLocationAtSplinePoint` _spline_3 _index_2 "Local") (`SplineComponent.GetTangentAtSplinePoint` _spline_3 _index_2 "Local") (`SplineComponent.GetLocationAtSplinePoint` _spline_2 _returnvalue_3 "Local") (`SplineComponent.GetTangentAtSplinePoint` _spline_2 _returnvalue_3 "Local") true)))))
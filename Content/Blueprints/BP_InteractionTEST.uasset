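; BP_InteractionTEST is a test actor for an interaction system, exposing highlight, interact and interactability hooks.
; SetHighlight toggles the M_Overlay overlay material on its Cube, highlighting it without replacing the base material.
; Interact only prints a debug message, and IsInteractable returns the CanInteract variable.
; Begin Play, overlap and Tick are empty, and a leftover highlight debug print branch is disconnected.
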(event `/Game/Blueprints/Interfaces/BPI_Interatable.SetHighlight`
  (params (Show :type Boolean))
  (`MeshComponent.SetOverlayMaterial` (`self.Cube`) (select `bool` Show :`true` "/Game/Materials/Overlay/M_Overlay.M_Overlay" :!type "MaterialInterface Object Reference") false 0))

(event `/Game/Blueprints/Interfaces/BPI_Interatable.Interact`
  (`KismetSystemLibrary.PrintString` "interacted"))

(fn `IsInteractable`
  (returns (Interactable :type Boolean))
  (return (`self.CanInteract`)))

(fn `UserConstructionScript`)
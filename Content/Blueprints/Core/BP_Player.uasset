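; First-person player character with Enhanced Input movement, look with optional Y inversion, interaction, and a godmode teleport to the next checkpoint.
; A camera-linked component tracks the current interactable, which receives the interact message.
; A timeline drives vertical camera head wobble, with rate and height scaled by walk speed.
; Possession toggles the input mapping context, while death and checkpoint queries go through a GameMode message interface.
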(event `self.ReceiveBeginPlay`
  (`self.SetupCamera`)
  (`self.HeadWobble`))

(event `HeadWobble`
  ;[0.776 0.001347 0.1345 0.5] Headwobble
  (bind (_direction _alpha) (`Timeline|Wobble`)
    (:`Update`
      (`TimelineComponent.SetPlayRate` (`self.Wobble`) (* (`self.HeadWobbleSpeed`) (`self.SpeedMapRange` 1.0 5.0)))
      (`SceneComponent.K2_SetRelativeLocation` (`self.Camera`) (`KismetMathLibrary.MakeVector` 0.0 0.0 (* _alpha (`self.HeadWobbleHight`) (`self.SpeedMapRange` 1.0 4.0))) false false))))

(event `PlayerDied`
  (bind _gamemode_ref (message `/Game/Blueprints/Interfaces/BPI_GameMode.MyGetGameMode` (`GameplayStatics.GetGameMode`)))
  (`/Game/Blueprints/Core/BP_GameMode.PlayerDeath` _gamemode_ref))

(event `self.ReceiveUnpossessed`
  (params (OldController :type "Controller Object Reference"))
  (`/Game/Blueprints/BPML_Generic.MyChangeMappingContext` false "/Game/Inputs/Player/IMC_Player.IMC_Player"))

(event `self.ReceivePossessed`
  (params (NewController :type "Controller Object Reference"))
  (`/Game/Blueprints/BPML_Generic.MyChangeMappingContext` true "/Game/Inputs/Player/IMC_Player.IMC_Player"))

(event `EnhancedInput|/Game/Inputs/Player/IA_Move`
  (params (ActionValue :type "Vector2D Structure") (ElapsedSeconds :type "Float (double-precision)") (TriggeredSeconds :type "Float (double-precision)") (InputAction :type "InputAction Object Reference" :default "/Game/Inputs/Player/IA_Move.IA_Move"))
  (bind (_returnvalue_roll _returnvalue_pitch _returnvalue_yaw) (`KismetMathLibrary.BreakRotator` (`self.GetControlRotation`)))
  (bind (_returnvalue_roll_2 _returnvalue_pitch_2 _returnvalue_yaw_2) (`KismetMathLibrary.BreakRotator` (`self.GetControlRotation`)))
  ;[0 0.7676 1 0.5] Move VorneHinten
  (:`Triggered`
    (`self.AddMovementInput` (`KismetMathLibrary.GetForwardVector` (`KismetMathLibrary.MakeRotator` 0.0 0.0 _returnvalue_yaw_2)) ActionValue_X)
    ;[0 0.7676 1 0.5] links  rechts
    (`self.AddMovementInput` (`KismetMathLibrary.GetRightVector` (`KismetMathLibrary.MakeRotator` 0.0 0.0 _returnvalue_yaw)) ActionValue_Y)))

(event `EnhancedInput|/Game/Inputs/Player/IA_Look`
  (params (ActionValue :type "Vector2D Structure") (ElapsedSeconds :type "Float (double-precision)") (TriggeredSeconds :type "Float (double-precision)") (InputAction :type "InputAction Object Reference" :default "/Game/Inputs/Player/IA_Look.IA_Look"))
  ;[0 1 0.5237 0.5] Look und y Invert
  (:`Triggered`
    (`self.AddControllerYawInput` (* ActionValue_X (`self.LookSensitivity`)))
    (`self.AddControllerPitchInput` (* ActionValue_Y (`self.LookSensitivity`) (`KismetMathLibrary.SelectInt` -1 1 (`self.InvertY`))))))

(event `EnhancedInput|/Game/Inputs/Player/IA_Interact`
  (params (ActionValue :type Boolean) (ElapsedSeconds :type "Float (double-precision)") (TriggeredSeconds :type "Float (double-precision)") (InputAction :type "InputAction Object Reference" :default "/Game/Inputs/Player/IA_Interact.IA_Interact"))
  ;[0.3105 1 0 0.5] INTERACT
  (:`Started`
    (message `/Game/Blueprints/Interfaces/BPI_Interatable.Interact` (`/Game/Blueprints/Components/BPC_CheckForInteractables.CurrentInteractable` (`self.Check for Interactables`)) self)))

(event `EnhancedInput|/Game/Inputs/Player/IA_TP`
  (params (ActionValue :type Boolean) (ElapsedSeconds :type "Float (double-precision)") (TriggeredSeconds :type "Float (double-precision)") (InputAction :type "InputAction Object Reference" :default "/Game/Inputs/Player/IA_TP.IA_TP"))
  ;[0.8797 1 0.003789 0.5] TP godmode
  (:`Started`
    (bind _gamemode_ref (message `/Game/Blueprints/Interfaces/BPI_GameMode.MyGetGameMode` (`GameplayStatics.GetGameMode`)))
    (bind _checkpointtransform (`/Game/Blueprints/Core/BP_GameMode.GetNextCheckpoint` _gamemode_ref))
    (`self.K2_SetActorLocation` (.location _checkpointtransform))
    (`Controller.SetControlRotation` (`GameplayStatics.GetPlayerController` 0) (.rotation _checkpointtransform))))

(fn `ChangeMappingContext`
  (params (Activate :type Boolean))
  (bind _returnvalue (pcsubsystem `EnhancedInputLocalPlayerSubsystem` (`GameplayStatics.GetPlayerController` 0)))
  (if Activate
    (`EnhancedInputSubsystemInterface.AddMappingContext` _returnvalue "/Game/Inputs/Player/IMC_Player.IMC_Player" 0 (struct))
    (else
      (`EnhancedInputSubsystemInterface.RemoveMappingContext` _returnvalue "/Game/Inputs/Player/IMC_Player.IMC_Player" (struct)))))

(fn `MyGetPlayer`
  (returns (`Player Ref` :type "/Game/Blueprints/Core/BP_Player Object Reference"))
  (return self))

(fn `SetupCamera`
  (bind _returnvalue (`GameplayStatics.GetPlayerCameraManager` 0))
  (set `PlayerCameraManager.ViewPitchMin` (`self.View Pitch Min`) _returnvalue)
  (set `PlayerCameraManager.ViewPitchMax` (`self.View Pitch Max`) _returnvalue))

(fn `UserConstructionScript`
  (bind _returnvalue (`AddComponent|NODE_AddBPC_CheckForInteractables-0` :`Camera` (`self.Camera`)))
  (set `self.Check for Interactables` _returnvalue))
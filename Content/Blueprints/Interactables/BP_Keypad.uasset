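; Interactable keypad pawn for code entry that plays an optional level sequence when the correct code is confirmed.
; Interact blends possession to the keypad and enables its input mapping; exiting restores the previous pawn.
; Directional input moves a wrapping highlight across the button grid, and pressing animates the button, appending digits, confirming or deleting.
; A wrong code or delete runs a color timeline before clearing; success exits and disables further interaction.
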(event `self.ReceiveBeginPlay`
  (`self.setup parameters`))

(event `setup parameters`
  ; anim speed
  (`|ExecutionSequence`
    (:`then_0`
      (`TimelineComponent.SetPlayRate` (`self.ButtonAnim`) (`self.speedanim`)))))

(event `/Game/Blueprints/Interfaces/BPI_Interatable.SetHighlight`
  (params (Show :type Boolean))
  ; set highlight
  (`MeshComponent.SetOverlayMaterial` (`self.basepad`) (select `bool` Show :`true` "/Game/Materials/Overlay/M_Overlay.M_Overlay" :!type "MaterialInterface Object Reference") false 0))

(event `/Game/Blueprints/Interfaces/BPI_Interatable.Interact`
  (params (LastPossess :type "Pawn Object Reference"))
  ; interact
  (set `self.Last Possess REF` LastPossess)
  (`/Game/Blueprints/BPML_Generic.MySmoothPossess` self)
  (`/Game/Blueprints/BPML_Generic.MyChangeMappingContext` true "/Game/Inputs/Keypad/IMC_Keypad.IMC_Keypad")
  (`self.Change Button Highlight` (`self.CurrentButton`)))

(event `Exit Keypad`
  ; exit keypad
  (`/Game/Blueprints/BPML_Generic.MySmoothPossess` (`self.Last Possess REF`))
  (`/Game/Blueprints/BPML_Generic.MyChangeMappingContext` false "/Game/Inputs/Keypad/IMC_Keypad.IMC_Keypad")
  (`self.Change Button Highlight` (`self.CurrentButton`) false))

(event `Change Button Highlight`
  (params (ButtonPosition :type Integer) (Enable :type Boolean :default true))
  ; change highlight
  (`/Game/Blueprints/Components/BPC_Keypadbutton.SetButtonHighlight` (`|GetArrayItem` (`self.ButtonList`) ButtonPosition) Enable))

(event `AnimateButtonPress`
  ; button anim
  (`/Engine/EditorBlueprintResources/StandardMacros.IsValid` (`self.LastPressedButton`)
    (:`Is Valid`
      (`SceneComponent.K2_SetRelativeLocation` (`self.LastPressedButton`) (0.0 0.0 0.0) false false))
    (:`Is Not Valid`
      _))
  (set `self.LastPressedButton` (`|GetArrayItem` (`self.ButtonList`) (`self.CurrentButton`)))
  (bind (_direction _alpha) (`Timeline|ButtonAnim` :!via `PlayFromStart`)
    (:`Update`
      (`SceneComponent.K2_SetRelativeLocation` (`self.LastPressedButton`) (`KismetMathLibrary.VLerp` (0.0 0.0 0.0) (4.0 0.0 0.0) _alpha) false false))))

(event `EnhancedInput|/Game/Inputs/Keypad/IA_Back`
  (params (ActionValue :type Boolean) (ElapsedSeconds :type "Float (double-precision)") (TriggeredSeconds :type "Float (double-precision)") (InputAction :type "InputAction Object Reference" :default "/Game/Inputs/Keypad/IA_Back.IA_Back"))
  (:`Triggered`
    (`self.Exit Keypad`)))

(event `EnhancedInput|/Game/Inputs/Keypad/IA_Right`
  (params (ActionValue :type Boolean) (ElapsedSeconds :type "Float (double-precision)") (TriggeredSeconds :type "Float (double-precision)") (InputAction :type "InputAction Object Reference" :default "/Game/Inputs/Keypad/IA_Right.IA_Right"))
  ;[0.01998 0.594 0.974 0.5] Right
  (:`Started`
    (`self.Change Button Highlight` (`self.CurrentButton`) false)
    (set `self.CurrentButton` (+ (`self.CurrentButton`) 1))
    (if (== (`self.CurrentButton`) (`KismetArrayLibrary.Array_Length` (`self.ButtonList`)))
      (set `self.CurrentButton` 0))
    (`self.Change Button Highlight` (`self.CurrentButton`))))

(event `EnhancedInput|/Game/Inputs/Keypad/IA_Left`
  (params (ActionValue :type Boolean) (ElapsedSeconds :type "Float (double-precision)") (TriggeredSeconds :type "Float (double-precision)") (InputAction :type "InputAction Object Reference" :default "/Game/Inputs/Keypad/IA_Left.IA_Left"))
  ;[1 0.1158 0.3191 0.5] Left
  (:`Started`
    (`self.Change Button Highlight` (`self.CurrentButton`) false)
    (set `self.CurrentButton` (- (`self.CurrentButton`) 1))
    (if (< (`self.CurrentButton`) 0)
      (set `self.CurrentButton` (- (`KismetArrayLibrary.Array_Length` (`self.ButtonList`)) 1)))
    (`self.Change Button Highlight` (`self.CurrentButton`))))

(event `EnhancedInput|/Game/Inputs/Keypad/IA_Down`
  (params (ActionValue :type Boolean) (ElapsedSeconds :type "Float (double-precision)") (TriggeredSeconds :type "Float (double-precision)") (InputAction :type "InputAction Object Reference" :default "/Game/Inputs/Keypad/IA_Down.IA_Down"))
  ;[0.09129 1 0.1674 0.5] down
  (:`Started`
    (`self.Change Button Highlight` (`self.CurrentButton`) false)
    (set `self.CurrentButton` (+ (`self.CurrentButton`) (`self.ButtonsPerRow`)))
    (if (>= (`self.CurrentButton`) (`KismetArrayLibrary.Array_Length` (`self.ButtonList`)))
      (set `self.CurrentButton` (- (`self.CurrentButton`) (`KismetArrayLibrary.Array_Length` (`self.ButtonList`)))))
    (`self.Change Button Highlight` (`self.CurrentButton`))))

(event `EnhancedInput|/Game/Inputs/Keypad/IA_Up`
  (params (ActionValue :type Boolean) (ElapsedSeconds :type "Float (double-precision)") (TriggeredSeconds :type "Float (double-precision)") (InputAction :type "InputAction Object Reference" :default "/Game/Inputs/Keypad/IA_Up.IA_Up"))
  ;[1 0.9095 0.05709 0.5] up
  (:`Started`
    (`self.Change Button Highlight` (`self.CurrentButton`) false)
    (set `self.CurrentButton` (- (`self.CurrentButton`) (`self.ButtonsPerRow`)))
    (if (< (`self.CurrentButton`) 0)
      (set `self.CurrentButton` (+ (`self.CurrentButton`) (`KismetArrayLibrary.Array_Length` (`self.ButtonList`)))))
    (`self.Change Button Highlight` (`self.CurrentButton`))))

(event `Delete Code`
  ;[1 0.1094 0.1094 0.5] Delete Code
  (`self.DisableInput` null)
  (bind (_direction _alpha) (`Timeline|WrongCodeAnim` :!via `PlayFromStart`)
    (:`Update`
      (`TextRenderComponent.SetTextRenderColor` (`self.TXT_CurrentCode`) (`KismetMathLibrary.Conv_LinearColorToColor` _alpha)))
    (:`Finished`
      (set `self.Current Code` "")
      (`TextRenderComponent.K2_SetText` (`self.TXT_CurrentCode`) "0000")
      (`self.EnableInput` null))))

(event `EnhancedInput|/Game/Inputs/Player/IA_Interact`
  (params (ActionValue :type Boolean) (ElapsedSeconds :type "Float (double-precision)") (TriggeredSeconds :type "Float (double-precision)") (InputAction :type "InputAction Object Reference" :default "/Game/Inputs/Player/IA_Interact.IA_Interact"))
  (bind _levelsequence_to_play (`self.LevelSequence to play`))
  (bind _content (`/Game/Blueprints/Components/BPC_Keypadbutton.Content` (`|GetArrayItem` (`self.ButtonList`) (`self.CurrentButton`))))
  (:`Started`
    (`self.AnimateButtonPress`)
    (switch `string` _content
      (:`Default`
        ;[0.9635 0.9356 0.2679 0.5] Numbers
        (if (< (`KismetStringLibrary.Len` (`self.Current Code`)) (`KismetStringLibrary.Len` (`self.Wanted Code`)))
          (bind _output_get (set `self.Current Code` (`KismetStringLibrary.Concat_StrStr` (`self.Current Code`) _content)))
          (`TextRenderComponent.K2_SetText` (`self.TXT_CurrentCode`) (`KismetTextLibrary.Conv_StringToText` _output_get))))
      (:`confirm`
        ;[0.01128 0.8976 0.07538 0.5] CorrectCode
        (if (`KismetStringLibrary.EqualEqual_StrStr` (`self.Current Code`) (`self.Wanted Code`))
          (`TextRenderComponent.SetTextRenderColor` (`self.TXT_CurrentCode`) (`KismetMathLibrary.LinearColor_ToRGBE` (struct :`R` 0.056156 :`G` 1.0 :`A` 1.0)))
          (`self.Exit Keypad`)
          (set `self.CanInteractIsActivated` false)
          (`/Engine/EditorBlueprintResources/StandardMacros.IsValid` _levelsequence_to_play
            (:`Is Valid`
              (`MovieSceneSequencePlayer.Play` (`LevelSequenceActor.SequencePlayer` _levelsequence_to_play))))
          (else
            (`self.Delete Code`))))
      (:`delete`
        (`self.Delete Code`)))))

(fn `IsInteractable`
  (returns (Interactable :type Boolean))
  (return (`self.CanInteractIsActivated`)))

(fn `UserConstructionScript`
  (set `self.ButtonList` (`|MakeArray` (`self.BPC_Keypadbutton1`) (`self.BPC_Keypadbutton2`) (`self.BPC_Keypadbutton3`) (`self.BPC_Keypadbutton4`) (`self.BPC_Keypadbutton5`) (`self.BPC_Keypadbutton6`) (`self.BPC_Keypadbutton7`) (`self.BPC_Keypadbutton8`) (`self.BPC_Keypadbutton9`) (`self.BPC_KeypadbuttonDEL`) (`self.BPC_Keypadbutton0`) (`self.BPC_KeypadbuttonOK`))))
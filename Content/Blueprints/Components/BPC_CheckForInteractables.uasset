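; Actor component that detects the interactable object the owning player-controlled pawn is looking at and highlights it.
; Every tick, a small sphere trace on the Visibility channel runs from the camera along its forward vector, with per-frame debug drawing.
; Hits implementing BPI_Interatable that report as interactable become CurrentInteractable.
; Highlight messages switch on for a new target and off for the previous one or when none qualifies.
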(event `self.ReceiveTick`
  (params (DeltaSeconds :type "Float (single-precision)"))
  (`self.InteractableCheck`))

(event `InteractableCheck`
  (bind _camera (`self.Camera`))
  (bind _returnvalue (`SceneComponent.K2_GetComponentLocation` _camera))
  (bind _outhit (`KismetSystemLibrary.SphereTraceSingle` :`Start` _returnvalue :`End` (+ _returnvalue (* (`SceneComponent.GetForwardVector` _camera) (`self.Interaction Distance`))) :`Radius` 2.0 :`TraceChannel` "TraceTypeQuery1" :`DrawDebugType` "ForOneFrame"))
  (bind (_bblockinghit _binitialoverlap _time _distance _location _impactpoint _normal _impactnormal _physmat _hitactor) (`GameplayStatics.BreakHitResult` _outhit))
  (bind _interactable (message `/Game/Blueprints/Interfaces/BPI_Interatable.IsInteractable` _hitactor))
  (if (and _interactable (`KismetSystemLibrary.DoesImplementInterface` _hitactor "/Game/Blueprints/Interfaces/BPI_Interatable.BPI_Interatable_C") (`Pawn.IsPlayerControlled` (cast `Pawn` (`self.GetOwner`) :!pure true)))
    (if (not (== (`self.CurrentInteractable`) _hitactor))
      (message `/Game/Blueprints/Interfaces/BPI_Interatable.SetHighlight` (`self.CurrentInteractable`) false)
      (bind _output_get (set `self.CurrentInteractable` _hitactor))
      (message `/Game/Blueprints/Interfaces/BPI_Interatable.SetHighlight` _output_get true))
    (else
      (`/Engine/EditorBlueprintResources/StandardMacros.IsValid` (`self.CurrentInteractable`)
        (:`Is Valid`
          (message `/Game/Blueprints/Interfaces/BPI_Interatable.SetHighlight` (`self.CurrentInteractable`) false)
          (set `self.CurrentInteractable` null))))))